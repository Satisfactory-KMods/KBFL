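; KBFL default subsystem that opens the cheat player menu from a key binding.
; On begin play it enables input on the FG player controller.
; When the open-menu input action triggers, it checks that host cheat mode is enabled and the controller and HUD are valid, then opens the cheat player widget as an interact UI with itself as the interact object.
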(event `self.ReceiveBeginPlay`
  (`parent.ReceiveBeginPlay`)
  (`self.EnableInput` (`KBFL_Player.GetFGController`)))

(event `EnhancedInput|/KBFL/IA_KBFL_OpenMenu`
  (params (ActionValue :type Boolean) (ElapsedSeconds :type "Float (double-precision)") (TriggeredSeconds :type "Float (double-precision)") (InputAction :type "InputAction Object Reference" :default "/KBFL/IA_KBFL_OpenMenu.IA_KBFL_OpenMenu"))
  (bind _returnvalue (`KBFL_Player.GetFGController`))
  (:`Triggered`
    (if (`KBFLUtilSubsystem.bIsHostEnableCheatMode` (`KBFLUtilSubsystem.Get` null))
      (`/Engine/EditorBlueprintResources/StandardMacros.IsValid` _returnvalue
        (:`Is Valid`
          (bind _outhud (`/Game/FactoryGame/Interface/UI/HUDHelpers/BPFL_HudHelperBadRef.GetBPHUD` _returnvalue))
          (`/Engine/EditorBlueprintResources/StandardMacros.IsValid` _outhud
            (:`Is Valid`
              (`FGHUD.OpenInteractUI` _outhud "/KBFL/Utils/CheatBuilding/Widget_CheatPlayerUI.Widget_CheatPlayerUI_C" self))))))))

(fn `UserConstructionScript`)