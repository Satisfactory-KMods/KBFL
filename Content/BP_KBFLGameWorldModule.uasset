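; Game world module Blueprint, KBFL by its name, that applies "easy nodes" processing to research trees when the world module initializes.
; On the Initialization lifecycle phase, after the parent call, it checks UseEasyNodes and runs ApplyEasyNodes.
; That function copies MResearchTrees into CachedForApply and passes it to EasyNodesLines.
; UseEasyNodes and IsAdaEnable both return true, though IsAdaEnable is not called here.
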(event `self.K2_OnLifecycleEvent`
  (params (Phase :type "ELifecyclePhase Enum" :default "CONSTRUCTION"))
  (`parent.K2_OnLifecycleEvent` Phase)
  (switch `ELifecyclePhase` Phase
    (:`INITIALIZATION`
      (if (`self.UseEasyNodes`)
        (`self.ApplyEasyNodes`)))))

(fn `ApplyEasyNodes`
  (locals (CachedForApply :type "Array of FGResearchTree Class Reference"))
  (bind _output_get (set `local.CachedForApply` (`self.mResearchTrees`)))
  (`/KBFL/BFL/KBFL_BP_EsayNodes.EasyNodes_Lines` _output_get))

(fn `IsAdaEnable`
  (returns (Value :type Boolean))
  (return true))

(fn `UseEasyNodes`
  (returns (Value :type Boolean))
  (return true))