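; Base resource node actor that, on BeginPlay, re-links resource extractors to replacement nodes through KBFL helpers.
; A non-persistent node finds an overlapping persistent node of its class, traces upward to reassign extractors to it, then destroys itself and notifies the node subsystem that spawning finished.
; A persistent, already-checked node waits briefly, then box-traces upward and assigns any extractor hit to its stored new-node reference.
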(event `self.ReceiveBeginPlay`
  (bind _returnvalue (`self.K2_GetActorLocation`))
  (bind _returnvalue_2 (`self.K2_GetActorLocation`))
  (bind _array (`|MakeArray` "ObjectTypeQuery1" "ObjectTypeQuery2" "ObjectTypeQuery3" "ObjectTypeQuery9" :!type "EObjectTypeQuery Enum"))
  (bind _array_2 (`|MakeArray` self :!type "Actor Object Reference"))
  (`parent.ReceiveBeginPlay`)
  (if (`self.mPresistent`)
    (if (`self.mWasChecked`)
      (`KismetSystemLibrary.Delay` 0.2)
      (bind _outhits (`KismetSystemLibrary.BoxTraceMultiForObjects` _returnvalue (+ _returnvalue (`KismetMathLibrary.MakeVector` 0.0 0.0 (`self.mUpperPerCheckRange`))) (100.0 100.0 100.0) (struct) (`|MakeArray` "ObjectTypeQuery1" "ObjectTypeQuery2" "ObjectTypeQuery3" "ObjectTypeQuery9" :!type "EObjectTypeQuery Enum") false (`|MakeArray` self)))
      (for _array_element _outhits
        (bind (_bblockinghit _binitialoverlap _time _distance _location _impactpoint _normal _impactnormal _physmat _hitactor) (`GameplayStatics.BreakHitResult` _array_element))
        (if _bblockinghit
          (`/Engine/EditorBlueprintResources/StandardMacros.IsValid` _hitactor
            (:`Is Valid`
              (bind _asfgbuildable_resource_extractor_base (cast `FGBuildableResourceExtractorBase` _hitactor))
              (`KBFL_Util.KBFL_SetResourceNodeToExtractor` _asfgbuildable_resource_extractor_base (`self.mNewNode`)))))))
    (else
      (bind _outactors (`KismetSystemLibrary.SphereOverlapActors` _returnvalue_2 50.0 _array (`GameplayStatics.GetObjectClass` self) _array_2))
      (for _array_element_2 _outactors
        (bind _asbp_resource_node_base (cast `/Game/ResourceNodeActors/BP_ResourceNodeBase` _array_element_2))
        (if (`/Game/ResourceNodeActors/BP_ResourceNodeBase.mPresistent` _asbp_resource_node_base)
          (set `self.mNewNode` _asbp_resource_node_base)))
      (`/Engine/EditorBlueprintResources/StandardMacros.IsValid` (`self.mNewNode`)
        (:`Is Valid`
          (bind _outhits_2 (`KismetSystemLibrary.LineTraceMultiForObjects` _returnvalue_2 (+ _returnvalue_2 (0.0 0.0 5000.0)) _array false _array_2))
          (for _array_element_3 _outhits_2
            (bind (_bblockinghit_2 _binitialoverlap_2 _time_2 _distance_2 _location_2 _impactpoint_2 _normal_2 _impactnormal_2 _physmat_2 _hitactor_2) (`GameplayStatics.BreakHitResult` _array_element_3))
            (if _bblockinghit_2
              (`/Engine/EditorBlueprintResources/StandardMacros.IsValid` _hitactor_2
                (:`Is Valid`
                  (bind _asfgbuildable_resource_extractor_base_2 (cast `FGBuildableResourceExtractorBase` _hitactor_2))
                  (`KBFL_Util.KBFL_SetResourceNodeToExtractor` _asfgbuildable_resource_extractor_base_2 (`self.mNewNode`)))))))
        (:`Is Not Valid`
          _))
      (`self.K2_DestroyActor`)
      (`KBFLResourceNodeSubsystem.Server_FinishedSpawningNodes` (subsystem `KBFLResourceNodeSubsystem`)))))

(fn `UserConstructionScript`
  (`parent.UserConstructionScript`))